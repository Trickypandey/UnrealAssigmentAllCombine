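; BP_DynamicPawnCOntroller is a Blueprint that shows pawn attributes as debug text.
; Its DisplayAttributes event receives an attribute asset and prints its speed, health and jump height as labeled strings.
; BeginPlay, Tick and the construction script are empty, and nothing in this Blueprint calls the event or applies the values to a pawn.
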(event EventBeginPlay)

(event EventTick
  (params (DeltaSeconds :type Float%20%28single-precision%29)))

(event EventDisplayAttributes
  (params (AttributeAsset :type Pawn%20Attribute%20Asset%20Object%20Reference))
  (Development|PrintString (Utilities|String|Append "Speed: " (Utilities|String|ToString(Float) (Variables|/Script/Assigment1_2.PawnAttributeAsset|GetSpeed AttributeAsset))))
  (Development|PrintString (Utilities|String|Append "Health:" (Utilities|String|ToString(Integer) (Variables|/Script/Assigment1_2.PawnAttributeAsset|GetHealth AttributeAsset))))
  (Development|PrintString (Utilities|String|Append "Jump Height" (Utilities|String|ToString(Float) (Variables|/Script/Assigment1_2.PawnAttributeAsset|GetJumpHeight AttributeAsset)))))

(fn ConstructionScript)